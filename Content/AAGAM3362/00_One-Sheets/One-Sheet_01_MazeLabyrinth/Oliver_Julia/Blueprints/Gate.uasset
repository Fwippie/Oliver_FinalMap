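; Gate Blueprint with a push button that the player presses with Interact while nearby.
; Box overlaps toggle input and a Gate node that filters presses, though begin and end cast to different character classes.
; A press runs a timeline sliding the button inward and plays the gate sound once.
; A separate OpenDoor event rotates the gate by timeline, with no caller in this file.
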(event OnComponentBeginOverlap(Box)
  (params (OverlappedComponent :type Primitive%20Component%20Object%20Reference) (OtherActor :type Actor%20Object%20Reference) (OtherComp :type Primitive%20Component%20Object%20Reference) (OtherBodyIndex :type Integer) (bFromSweep :type Boolean) (SweepResult :type Hit%20Result%20Structure%20%28by%20ref%29))
  ;[1 1 1] Hit "E" to open door if player is close enough
  (Utilities|Casting|CastToFirstPersonCharacter_h OtherActor)
  (Input|EnableInput (Game|GetPlayerController 0))
  (Utilities|FlowControl|Gate true) ; enters at Open
)

(event OnComponentEndOverlap(Box)
  (params (OverlappedComponent :type Primitive%20Component%20Object%20Reference) (OtherActor :type Actor%20Object%20Reference) (OtherComp :type Primitive%20Component%20Object%20Reference) (OtherBodyIndex :type Integer))
  ;[1 1 1] Hit "E" to open door if player is close enough
  (Utilities|Casting|CastToFirstPersonCharacter OtherActor)
  (Input|DisableInput (Game|GetPlayerController 0))
  (Utilities|FlowControl|Gate true) ; enters at Close
)

(event Custom|OpenDoor
  ;[1 1 1] Open/Close Door
  (bind _newtrack_0 (Timeline|Door%20Timeline Play)
    (:Update
      (Transformation|SetRelativeRotation (Variables|Default|GetGate) (Math|Rotator|MakeRotator 0.0 0.0 (Math|Float|Lerp (Variables|Default|Getclose%20angle) (Variables|Default|Getdoor%20open%20angle) _newtrack_0)) false false))))

(event Input|ActionEvents|InputActionInteract
  (params (Key :type Key%20Structure :default "None"))
  ;[1 1 1] Hit "E" to open door if player is close enough
  (:Pressed
    (Utilities|FlowControl|Gate true
      (:Exit
        ;[1 1 1] Push Button
        (|ButtonPressAnimation)))))

(fn ConstructionScript
  (Transformation|SetRelativeTransform (Variables|Default|GetButton) (Variables|Default|GetButton%20Transform) false false))